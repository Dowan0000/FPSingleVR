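; BP_Character is a character Blueprint that links to the main UI widget to refresh its gold display.
; On BeginPlay it calls the parent, then finds BP_WidgetActor and caches its widget as BP_MainWidget.
; UpdateGoldWidget forwards to UpdateGold on that cached widget.
; The PressB input action prints a debug string and plays force feedback on the first player controller.
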(event EventBeginPlay
  (|CallParentFunction)
  (bind _returnvalue (Actor|GetActorOfClass "/Game/_Game/Widgets/BP_WidgetActor.BP_WidgetActor_C"))
  (bind _asbp_main_widget (Utilities|Casting|CastToBP_MainWidget (UserInterface|GetWidget (Variables|/Game/_Game/Widgets/BP_WidgetActor.BP_WidgetActor_C|GetWidget _returnvalue))))
  (Variables|Default|SetAs%20BP%20Main%20Widget _asbp_main_widget))

(event EventUpdateGoldWidget
  (Default|UpdateGold (Variables|Default|GetAs%20BP%20Main%20Widget)))

(event Input|ActionEvents|InputActionPressB
  (params (Key :type Key%20Structure :default "None"))
  (:Pressed
    (Development|PrintString "bbbbbbbbbbbbbbbbbbb")
    (Game|Feedback|ClientPlayForceFeedback (Game|GetPlayerController 0) "/Game/_Game/Character/ForceFeedbackEffect.ForceFeedbackEffect" "None" false false false)))

(fn ConstructionScript)