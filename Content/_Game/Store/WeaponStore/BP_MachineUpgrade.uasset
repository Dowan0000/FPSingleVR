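; BP_MachineUpgrade is a store station for machine upgrades, built on a parent Blueprint that handles the base overlap logic.
; When the box overlap begins, it runs the parent handler, casts the StoreWidget to WBP_MachineUpgradeStroe, caches it, passes it the Character and shows its UpgradeBox.
; When the overlap ends, it collapses the UpgradeBox and clears the widget's Character reference if the cached widget is valid.
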(event EventBeginPlay)

(event EventBoxBeginOverlap
  (params (OverlappedComponent :type Primitive%20Component%20Object%20Reference) (OtherActor :type Actor%20Object%20Reference) (OtherComp :type Primitive%20Component%20Object%20Reference) (OtherBodyIndex :type Integer) (bFromSweep :type Boolean) (SweepResult :type Hit%20Result%20Structure%20%28by%20ref%29))
  (|CallParentFunction OverlappedComponent OtherActor OtherComp OtherBodyIndex bFromSweep SweepResult)
  (bind _aswbp_machine_upgrade_stroe (Utilities|Casting|CastToWBP_MachineUpgradeStroe (UserInterface|GetWidget (Variables|Default|GetStoreWidget))))
  (Variables|Default|SetAs%20WBP%20Machine%20Upgrade%20Stroe _aswbp_machine_upgrade_stroe)
  (Variables|/Game/_Game/Store/WeaponStore/WBP_MachineUpgradeStroe.WBP_MachineUpgradeStroe_C|SetCharacter _aswbp_machine_upgrade_stroe (Variables|Default|GetCharacter))
  (Widget|SetVisibility (Variables|/Game/_Game/Store/WeaponStore/WBP_MachineUpgradeStroe.WBP_MachineUpgradeStroe_C|GetUpgradeBox _aswbp_machine_upgrade_stroe) "Visible"))

(event EventBoxEndOverlap
  (params (OverlappedComponent :type Primitive%20Component%20Object%20Reference) (OtherActor :type Actor%20Object%20Reference) (OtherComp :type Primitive%20Component%20Object%20Reference) (OtherBodyIndex :type Integer))
  (bind _as_wbp_machine_upgrade_stroe (Variables|Default|GetAs%20WBP%20Machine%20Upgrade%20Stroe))
  (|CallParentFunction OverlappedComponent OtherActor OtherComp OtherBodyIndex)
  (Utilities|IsValid _as_wbp_machine_upgrade_stroe
    (:Is%20Valid
      (Widget|SetVisibility (Variables|/Game/_Game/Store/WeaponStore/WBP_MachineUpgradeStroe.WBP_MachineUpgradeStroe_C|GetUpgradeBox _as_wbp_machine_upgrade_stroe) "Collapsed")
      (Variables|/Game/_Game/Store/WeaponStore/WBP_MachineUpgradeStroe.WBP_MachineUpgradeStroe_C|SetCharacter _as_wbp_machine_upgrade_stroe 0))))

(fn ConstructionScript)