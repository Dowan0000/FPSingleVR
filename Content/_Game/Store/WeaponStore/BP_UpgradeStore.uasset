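; BP_UpgradeStore is an upgrade store in the weapon store set, showing its UI through the StoreWidget component.
; On box begin overlap it casts the widget to WBP_UpgradeStroe, caches it, passes in the Character and makes UpgradeBox visible.
; On box end overlap it clears the widget's Character but sets UpgradeBox to Visible again rather than hiding it.
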(event EventBeginPlay)

(event EventBoxBeginOverlap
  (params (OverlappedComponent :type Primitive%20Component%20Object%20Reference) (OtherActor :type Actor%20Object%20Reference) (OtherComp :type Primitive%20Component%20Object%20Reference) (OtherBodyIndex :type Integer) (bFromSweep :type Boolean) (SweepResult :type Hit%20Result%20Structure%20%28by%20ref%29))
  (bind _aswbp_upgrade_stroe (Utilities|Casting|CastToWBP_UpgradeStroe (UserInterface|GetWidget (Variables|Default|GetStoreWidget))))
  (Variables|Default|SetAs%20WBP%20Upgrade%20Stroe _aswbp_upgrade_stroe)
  (Variables|/Game/_Game/Store/WeaponStore/WBP_UpgradeStroe.WBP_UpgradeStroe_C|SetCharacter _aswbp_upgrade_stroe (Variables|Default|GetCharacter))
  (Widget|SetVisibility (Variables|/Game/_Game/Store/WeaponStore/WBP_UpgradeStroe.WBP_UpgradeStroe_C|GetUpgradeBox _aswbp_upgrade_stroe) "Visible"))

(event EventBoxEndOverlap
  (params (OverlappedComponent :type Primitive%20Component%20Object%20Reference) (OtherActor :type Actor%20Object%20Reference) (OtherComp :type Primitive%20Component%20Object%20Reference) (OtherBodyIndex :type Integer))
  (bind _as_wbp_upgrade_stroe (Variables|Default|GetAs%20WBP%20Upgrade%20Stroe))
  (Utilities|IsValid _as_wbp_upgrade_stroe
    (:Is%20Valid
      (Widget|SetVisibility (Variables|/Game/_Game/Store/WeaponStore/WBP_UpgradeStroe.WBP_UpgradeStroe_C|GetUpgradeBox _as_wbp_upgrade_stroe) "Visible")
      (Variables|/Game/_Game/Store/WeaponStore/WBP_UpgradeStroe.WBP_UpgradeStroe_C|SetCharacter (Variables|Default|GetAs%20WBP%20Upgrade%20Stroe) 0))))

(fn ConstructionScript)