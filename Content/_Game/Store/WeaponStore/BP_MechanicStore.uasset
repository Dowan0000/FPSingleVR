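; BP_MechanicStore is a mechanic store that shows its shop panel while its box overlap is active.
; On begin overlap it casts the StoreWidget's widget to WBP_MechanicStore, caches it, passes in the Character reference and makes MechanicBox visible.
; On end overlap it collapses MechanicBox and clears the widget's Character.
; Character is only read here, with no assignment in these graphs.
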(event EventBeginPlay)

(event EventBoxBeginOverlap
  (params (OverlappedComponent :type Primitive%20Component%20Object%20Reference) (OtherActor :type Actor%20Object%20Reference) (OtherComp :type Primitive%20Component%20Object%20Reference) (OtherBodyIndex :type Integer) (bFromSweep :type Boolean) (SweepResult :type Hit%20Result%20Structure%20%28by%20ref%29))
  (bind _aswbp_mechanic_store (Utilities|Casting|CastToWBP_MechanicStore (UserInterface|GetWidget (Variables|Default|GetStoreWidget))))
  (Variables|Default|SetAs%20WBP%20Mechanic%20Store _aswbp_mechanic_store)
  (Variables|/Game/_Game/Store/WeaponStore/WBP_MechanicStore.WBP_MechanicStore_C|SetCharacter _aswbp_mechanic_store (Variables|Default|GetCharacter))
  (Widget|SetVisibility (Variables|/Game/_Game/Store/WeaponStore/WBP_MechanicStore.WBP_MechanicStore_C|GetMechanicBox _aswbp_mechanic_store) "Visible"))

(event EventBoxEndOverlap
  (params (OverlappedComponent :type Primitive%20Component%20Object%20Reference) (OtherActor :type Actor%20Object%20Reference) (OtherComp :type Primitive%20Component%20Object%20Reference) (OtherBodyIndex :type Integer))
  (bind _as_wbp_mechanic_store (Variables|Default|GetAs%20WBP%20Mechanic%20Store))
  (Utilities|IsValid _as_wbp_mechanic_store
    (:Is%20Valid
      (Widget|SetVisibility (Variables|/Game/_Game/Store/WeaponStore/WBP_MechanicStore.WBP_MechanicStore_C|GetMechanicBox _as_wbp_mechanic_store) "Collapsed")
      (Variables|/Game/_Game/Store/WeaponStore/WBP_MechanicStore.WBP_MechanicStore_C|SetCharacter (Variables|Default|GetAs%20WBP%20Mechanic%20Store) 0))))

(fn ConstructionScript)