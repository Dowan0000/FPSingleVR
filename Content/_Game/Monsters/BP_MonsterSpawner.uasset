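; Monster spawner actor that places BP_Sprider monsters at its own transform and reports each one to the main HUD's monster count.
; BeginPlay spawns the first, caches BP_MainWidget from BP_WidgetActor's widget component, then starts a self-rescheduling Spawn Spider timer.
; At twenty spawns it resets its counter and hands off to Spawn Other, which is empty, so spawning ends there.
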(event EventBeginPlay
  (Game|SpawnActorfromClass "/Game/_Game/Monsters/Spider/BP_Sprider.BP_Sprider_C" (Transformation|GetActorTransform) "AdjustIfPossibleButAlwaysSpawn" 0 0)
  (Variables|Default|SetSpawned%20Monster (+ (Variables|Default|GetSpawned%20Monster) 1))
  (bind _returnvalue (Actor|GetActorOfClass "/Game/_Game/Widgets/BP_WidgetActor.BP_WidgetActor_C"))
  (bind _asbp_main_widget (Utilities|Casting|CastToBP_MainWidget (UserInterface|GetWidget (Variables|/Game/_Game/Widgets/BP_WidgetActor.BP_WidgetActor_C|GetWidget _returnvalue))))
  (bind _output_get (Variables|Default|SetAs%20BP%20Main%20Widget _asbp_main_widget))
  (Default|AddMonsterCount _output_get)
  (Utilities|Time|SetTimerbyFunctionName 0 "Spawn Spider" 5.0))

(fn ConstructionScript)

(fn SpawnSpider
  (Game|SpawnActorfromClass "/Game/_Game/Monsters/Spider/BP_Sprider.BP_Sprider_C" (Transformation|GetActorTransform) "AdjustIfPossibleButAlwaysSpawn" 0 0)
  (Variables|Default|SetSpawned%20Monster (+ (Variables|Default|GetSpawned%20Monster) 1))
  (Default|AddMonsterCount (Variables|Default|GetAs%20BP%20Main%20Widget))
  (if (>= (Variables|Default|GetSpawned%20Monster) 20)
    (Variables|Default|SetSpawned%20Monster 0)
    (Utilities|Time|SetTimerbyFunctionName 0 "Spawn Other" 5.0)
    (else
      (Utilities|Time|SetTimerbyFunctionName 0 "Spawn Spider" 5.0))))

(fn SpawnOther)